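; BP_SAMURAI is the player-controlled 2D samurai character, with side-scrolling movement, jumping and coin collection.
; BeginPlay adds its Enhanced Input mapping context, driving movement along world X and jumping, while acceleration direction flips control rotation yaw to face travel.
; ObtenerMoneda adds collected coins to the total and prints it on screen.
; ChequeoDeSalto tracks first and second jump flags, but nothing in this file calls it or reads PuedoSaltar.
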(event Input|EnhancedActionEvents|EnhancedInputActionIA_MOVERSE
  (params (ActionValue :type Float%20%28double-precision%29) (ElapsedSeconds :type Float%20%28double-precision%29) (TriggeredSeconds :type Float%20%28double-precision%29) (InputAction :type Input%20Action%20Object%20Reference :default "/Game/2D/CHARACTERS/INPUTS/IA_MOVERSE.IA_MOVERSE"))
  (bind _returnvalue (Pawn|GetController))
  (Pawn|Input|AddMovementInput "1.000000,0.000000,0.000000" ActionValue false)
  (Math|Float|CompareFloat (.x (Pawn|Components|CharacterMovement|GetCurrentAcceleration (Variables|Character|GetCharacterMovement))) 0.0
    (:>
      (Pawn|SetControlRotation _returnvalue (Math|Rotator|MakeRotator 0.0 0.0 0.0)))
    (:<
      (Pawn|SetControlRotation _returnvalue (Math|Rotator|MakeRotator 0.0 0.0 1.8e+02)))))

(event Input|EnhancedActionEvents|EnhancedInputActionIA_SALTAR
  (params (ActionValue :type Float%20%28double-precision%29) (ElapsedSeconds :type Float%20%28double-precision%29) (TriggeredSeconds :type Float%20%28double-precision%29) (InputAction :type Input%20Action%20Object%20Reference :default "/Game/2D/CHARACTERS/INPUTS/IA_SALTAR.IA_SALTAR"))
  (:Started
    (Character|Jump))
  (:Completed
    (Character|StopJumping)))

(event EventBeginPlay
  (bind _asplayer_controller (Utilities|Casting|CastToPlayerController (Pawn|GetController)))
  (Input|AddMappingContext (PlayerController|LocalPlayerSubsystems|GetEnhancedInputLocalPlayerSubsystem _asplayer_controller) "/Game/2D/CHARACTERS/INPUTS/MAPPING/IMC_SAMURAI.IMC_SAMURAI" 0 "(bIgnoreAllPressedKeysUntilRelease=True,bForceImmediately=False,bNotifyUserSettings=False)"))

(event EventObtenerMoneda
  (params (Moneda :type Integer))
  (bind _output_get (Variables|Default|SetMonedas (+ Moneda (Variables|Default|GetMonedas))))
  (Development|PrintString (Utilities|String|Append "Agarraste una moneda,  
tus monedas actuales son : " (Utilities|String|ToString(Integer) _output_get)) true true "(R=1.000000,G=0.000000,B=0.838870,A=1.000000)" 5.0))

(fn ConstructionScript)

(fn ChequeoDeSalto
  (if (Variables|Default|GetPrimer%20Salto%20hecho)
    (Variables|Default|SetPrimer%20Salto%20hecho false)
    (Variables|Default|SetPuedo%20Saltar? false)
    (else
      (Variables|Default|SetPrimer%20Salto%20hecho true))))